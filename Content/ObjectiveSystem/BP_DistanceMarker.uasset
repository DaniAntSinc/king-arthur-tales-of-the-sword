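; Objective marker actor that shows the player's distance to it in the quest UI.
; After a short delay on BeginPlay it loads the save game and destroys its widget component if the saved objective status differs from its objective number.
; Every Tick it writes the distance to the quest widget and all top-level 3D marker distance widgets.
; Overlap-based mission completion logic is present but disconnected, so never runs.
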(event `self.ReceiveBeginPlay`
  (bind _asbp_third_person_character (cast `/Game/BattleSystem/ThirdPerson/Blueprints/BP_ThirdPersonCharacter` (`GameplayStatics.GetPlayerCharacter` 0)))
  (set `self.PlayerRef` _asbp_third_person_character)
  (`KismetSystemLibrary.Delay` 1.0)
  (bind _returnvalue (`GameplayStatics.LoadGameFromSlot` "SaveSlot1"))
  (bind _assave_game_data (cast `/Game/BattleSystem/SaveGameData` _returnvalue))
  (if (not (== (`/Game/BattleSystem/SaveGameData.ObjectiveStatus` _assave_game_data) (`self.ObjectiveNumber`)))
    (`ActorComponent.K2_DestroyComponent` (`self.Widget`))))

(event `self.ReceiveTick`
  (params (DeltaSeconds :type "Float (single-precision)"))
  ;[0.15 0.1219 0 0.5] Calculate Distance to Player
  (`self.CalcultateDistanceToPlayer`))

(event `self.Trigger.OnComponentBeginOverlap`
  (params (OverlappedComponent :type "PrimitiveComponent Object Reference") (OtherActor :type "Actor Object Reference") (OtherComp :type "PrimitiveComponent Object Reference") (OtherBodyIndex :type Integer) (bFromSweep :type Boolean) (SweepResult :type "HitResult Structure (by ref)"))
  ; Objectives are updated based on Boss complation
)

(fn `CalcultateDistanceToPlayer`
  (bind _returnvalue (`KismetStringLibrary.Conv_IntToString` (`KismetMathLibrary.FTrunc` (/ (`KismetMathLibrary.Vector_Distance` (`self.K2_GetActorLocation`) (`self.K2_GetActorLocation` (`GameplayStatics.GetPlayerCharacter` 0))) 100.0))))
  (message `/Game/ObjectiveSystem/BPI_DistanceMarker.DistanceMarker` (`/Game/BattleSystem/ThirdPerson/Blueprints/BP_ThirdPersonCharacter.UI_QuestWidget` (`self.PlayerRef`)) (`KismetTextLibrary.Conv_StringToText` (`KismetStringLibrary.Concat_StrStr` _returnvalue (`self.NameUnits`))))
  (bind _foundwidgets (`WidgetBlueprintLibrary.GetAllWidgetsOfClass` "/Game/BattleSystem/UI/Widgets/UI_3DMarkerDistance.UI_3DMarkerDistance_C"))
  (for _array_element _foundwidgets
    (`TextBlock.SetText` (`/Game/BattleSystem/UI/Widgets/UI_3DMarkerDistance.Distance_Text` _array_element) (`KismetTextLibrary.Conv_StringToText` (`KismetStringLibrary.Concat_StrStr` _returnvalue " m")))))

(fn `UpdateCurrentMission`
  (params (CurrentMission :type String))
  (set `self.CurrentMission` CurrentMission)
  (set `TextBlock.Text` (`KismetTextLibrary.Conv_StringToText` (`self.CurrentMission`)) (`/Game/ObjectiveSystem/UI_Quests.CurrentMission_Text` (`/Game/BattleSystem/ThirdPerson/Blueprints/BP_ThirdPersonCharacter.UI_QuestWidget` (`self.PlayerRef`)))))

(fn `UserConstructionScript`)