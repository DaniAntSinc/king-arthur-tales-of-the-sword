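; Scene component that toggles an underwater post-process material when the player pawn is beneath water, ticking only on that pawn.
; On BeginPlay it finds an unbound post-process volume and uses the owner's camera, or itself, as the probe point.
; Each tick it traces upward through WorldDynamic objects for the water physical material.
; The result adds or removes the blendable by rebuilding the volume's settings, with a flag preventing repeat edits.
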(event `self.ReceiveBeginPlay`
  (if (`self.Is Player`)
    (`self.Init Volume`)
    (`self.Init Position Component`)
    (else
      (`self.SetComponentTickEnabled` false))))

(event `self.ReceiveTick`
  (params (DeltaSeconds :type "Float (single-precision)"))
  (`self.Detect Underwater`))

(fn `Add Material`
  (locals (`Post Process Materials` :type "Array of WeightedBlendable Structure"))
  (if (not (`self.Material Active`))
    (`/Engine/EditorBlueprintResources/StandardMacros.IsValid` (`self.Underwater PostProcess Material`)
      (:`Is Valid`
        (bind _output_get (set `local.Post Process Materials` (`.Array` (break `WeightedBlendables` (`.WeightedBlendables` (break `PostProcessSettings` (`PostProcessVolume.Settings` (`self.Post Process Volume`))))))))
        (for _array_element _output_get
          (if (== (`.Object` (break `WeightedBlendable` _array_element)) (`self.Underwater PostProcess Material`))
            (set `self.Material Active` true)
            (return)))
        (`KismetArrayLibrary.Array_Add` _output_get (make `WeightedBlendable` 1.0 (`self.Underwater PostProcess Material`)))
        (set `PostProcessVolume.Settings` (make `PostProcessSettings` :`WeightedBlendables` (make `WeightedBlendables` (`local.Post Process Materials`))) (`self.Post Process Volume`))
        (set `self.Material Active` true)))))

(fn `Detect Underwater`
  (bind _returnvalue (`self.K2_GetComponentLocation` (`self.Position Component`)))
  (bind _outhits (`KismetSystemLibrary.LineTraceMultiForObjects` _returnvalue (+ (`KismetMathLibrary.MakeVector` 0.0 0.0 10000.0) _returnvalue) (`|MakeArray` "ObjectTypeQuery2" :!type "EObjectTypeQuery Enum") false (`|MakeArray` (`GameplayStatics.GetPlayerPawn` 0) :!type "Actor Object Reference")))
  (for _array_element _outhits
    (if (== (`.PhysMat` (`GameplayStatics.BreakHitResult` _array_element)) (`self.Water Physical Material`))
      (`self.Add Material`)
      (return)))
  (`self.Remove Material`))

(fn `Init Position Component`
  (bind _returnvalue (`Actor.GetComponentByClass` (`self.GetOwner`) "/Script/Engine.CameraComponent"))
  (`/Engine/EditorBlueprintResources/StandardMacros.IsValid` _returnvalue
    (:`Is Valid`
      (set `self.Position Component` _returnvalue))
    (:`Is Not Valid`
      (set `self.Position Component` self))))

(fn `Init Volume`
  (bind _outactors (`GameplayStatics.GetAllActorsOfClass` "/Script/Engine.PostProcessVolume")) ; Possibly also use tag but using infinite extent check for simpliciy
  (for _array_element _outactors
    (if (`PostProcessVolume.bUnbound` _array_element)
      (set `self.Post Process Volume` _array_element)
      (break)))
  (`/Engine/EditorBlueprintResources/StandardMacros.IsValid` (`self.Post Process Volume`)
    (:`Is Valid`
      (`KismetSystemLibrary.PrintString` "Warning: Valid Outline Volume not Found!" true true (struct :`R` 1.0 :`G` 0.7909 :`A` 1.0)))))

(fn `Is Player`
  (returns (`Is Player` :type Boolean))
  (locals (NewLocalVar :type Boolean))
  (return (== (`self.GetOwner`) (`GameplayStatics.GetPlayerPawn` 0))))

(fn `Remove Material`
  (locals (`Post Process Materials` :type "Array of WeightedBlendable Structure"))
  (if (`self.Material Active`)
    (`/Engine/EditorBlueprintResources/StandardMacros.IsValid` (`self.Underwater PostProcess Material`)
      (:`Is Valid`
        (for _array_element (`.Array` (break `WeightedBlendables` (`.WeightedBlendables` (break `PostProcessSettings` (`PostProcessVolume.Settings` (`self.Post Process Volume`))))))
          (if (!= (`.Object` (break `WeightedBlendable` _array_element)) (`self.Underwater PostProcess Material`))
            (`KismetArrayLibrary.Array_Add` (`local.Post Process Materials`) _array_element)))
        (set `PostProcessVolume.Settings` (make `PostProcessSettings` :`WeightedBlendables` (make `WeightedBlendables` (`local.Post Process Materials`))) (`self.Post Process Volume`))
        (set `self.Material Active` false)))))