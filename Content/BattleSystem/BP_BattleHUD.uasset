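; BP_BattleHUD is the battle HUD actor that creates and owns the on-screen UI for battles.
; On BeginPlay it adds a layout widget to the viewport, pushes BattleHeadsUpDisplay onto its UI.Layer.GameMenu layer and caches that widget.
; Wrapper functions expose the layout's layer push and forward party unit additions and unit display requests to the cached widget, keeping callers off the widgets themselves.
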(event `self.ReceiveBeginPlay`
  (bind _returnvalue (`|CreateWidget` "/Game/BattleSystem/UI/Widgets/LayoutWidget.LayoutWidget_C" (`self.GetOwningPlayerController`)))
  (bind _output_get (set `self.Layout` _returnvalue))
  (`UserWidget.AddToViewport` _output_get 0)
  (bind _widget (`/Game/BattleSystem/UI/Widgets/LayoutWidget.PushToLayer` _output_get (struct :`TagName` "UI.Layer.GameMenu") "/Game/BattleSystem/UI/Widgets/Combat/BattleHeadsUpDisplay.BattleHeadsUpDisplay_C"))
  (bind _asbattle_heads_up_display (cast `/Game/BattleSystem/UI/Widgets/Combat/BattleHeadsUpDisplay` _widget))
  (set `self.HUD` _asbattle_heads_up_display))

(fn `AddPartyUnit`
  (params (Unit :type "/Game/BattleSystem/UnitBase Object Reference"))
  (`/Game/BattleSystem/UI/Widgets/Combat/BattleHeadsUpDisplay.AddPartyUnitToHUD` (`self.HUD`) Unit))

(fn `PushToLayer`
  (params (Layer :type "GameplayTag Structure") (WidgetClass :type "CommonActivatableWidget Class Reference"))
  (returns (Widget :type "CommonActivatableWidget Object Reference"))
  (bind _widget (`/Game/BattleSystem/UI/Widgets/LayoutWidget.PushToLayer` (`self.Layout`) Layer WidgetClass))
  (return _widget))

(fn `ShowUnit`
  (params (Unit :type "/Game/BattleSystem/UnitBase Object Reference"))
  (`/Game/BattleSystem/UI/Widgets/Combat/BattleHeadsUpDisplay.ShowUnit1` (`self.HUD`) Unit))

(fn `UserConstructionScript`)