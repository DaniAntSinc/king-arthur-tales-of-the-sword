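; Actor component that drives a custom depth stencil outline on one primitive component of its owner, for the battle system.
; On BeginPlay it defaults the target to the owner's first PrimitiveComponent unless one is already set through SetStencilTarget.
; SetEnabled toggles custom depth rendering and writes the stored stencil value or zero, while SetStencilValue stores a new value and applies it only while enabled.
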(event `self.ReceiveBeginPlay`
  (`self.Init Default Target`))

(fn `Init Default Target`
  (bind _returnvalue (`self.GetOwner`))
  (`/Engine/EditorBlueprintResources/StandardMacros.IsValid` (`self.Target`)
    (:`Is Not Valid`
      (`/Engine/EditorBlueprintResources/StandardMacros.IsValid` _returnvalue
        (:`Is Valid`
          (set `self.Target` (`Actor.GetComponentByClass` _returnvalue "/Script/Engine.PrimitiveComponent")))))))

(fn `Set Enabled`
  (params (Enable :type Boolean))
  (bind _target (`self.Target`))
  (set `self.Enabled` Enable)
  (`/Engine/EditorBlueprintResources/StandardMacros.IsValid` _target
    (:`Is Valid`
      (`PrimitiveComponent.SetCustomDepthStencilValue` _target (`KismetMathLibrary.SelectInt` (`self.Stencil Value`) 0 (`self.Enabled`)))
      (`PrimitiveComponent.SetRenderCustomDepth` _target (`self.Enabled`)))))

(fn `Set Stencil Target`
  (params (`Stencil Target Component` :type "PrimitiveComponent Object Reference"))
  (set `self.Target` `Stencil Target Component`))

(fn `Set Stencil Value`
  (params (NewParam :type Integer))
  (bind _target (`self.Target`))
  (bind _output_get (set `self.Stencil Value` NewParam))
  (if (`self.Enabled`)
    (`/Engine/EditorBlueprintResources/StandardMacros.IsValid` _target
      (:`Is Valid`
        (`PrimitiveComponent.SetCustomDepthStencilValue` _target _output_get)))))