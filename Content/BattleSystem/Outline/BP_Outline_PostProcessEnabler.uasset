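; Battle-system actor that installs an outline post-process material at runtime and drives its mask parameter.
; On BeginPlay it finds the first unbound PostProcessVolume, printing a warning if none exists, and creates a dynamic instance of the configured material.
; It appends that instance to a copy of the volume's blendables and writes the settings back.
; SetMask stores the mask and pushes it to the material; SetEnabled is an empty stub.
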(event `self.ReceiveBeginPlay`
  (`self.Init Volume`)
  (`self.Init Material`)
  (`self.Set Mask` (`self.Outline Mask`)))

(fn `Init Material`
  (locals (`Post Process Materials` :type "Array of WeightedBlendable Structure"))
  (bind _post_process_material (`self.Post Process Material`))
  (bind _outline_volume (`self.Outline Volume`))
  (`/Engine/EditorBlueprintResources/StandardMacros.IsValid` _post_process_material
    (:`Is Valid`
      (`/Engine/EditorBlueprintResources/StandardMacros.IsValid` _outline_volume
        (:`Is Valid`
          (bind _returnvalue (`KismetMaterialLibrary.CreateDynamicMaterialInstance` _post_process_material))
          (set `self.Dynamic Outline Material` _returnvalue)
          (bind _output_get (set `local.Post Process Materials` (`.Array` (break `WeightedBlendables` (`.WeightedBlendables` (break `PostProcessSettings` (`PostProcessVolume.Settings` _outline_volume)))))))
          (`KismetArrayLibrary.Array_Add` _output_get (make `WeightedBlendable` 1.0 (`self.Dynamic Outline Material`)))
          (set `PostProcessVolume.Settings` (make `PostProcessSettings` :`WeightedBlendables` (make `WeightedBlendables` (`local.Post Process Materials`))) _outline_volume))))))

(fn `Init Volume`
  (bind _outactors (`GameplayStatics.GetAllActorsOfClass` "/Script/Engine.PostProcessVolume")) ; Possibly also use tag but using infinite extent check for simpliciy
  (for _array_element _outactors
    (if (`PostProcessVolume.bUnbound` _array_element)
      (set `self.Outline Volume` _array_element)
      (break)))
  (`/Engine/EditorBlueprintResources/StandardMacros.IsValid` (`self.Outline Volume`)
    (:`Is Not Valid`
      (`KismetSystemLibrary.PrintString` "Warning: Valid Outline Volume not Found!" true true (struct :`R` 1.0 :`G` 0.7909 :`A` 1.0)))))

(fn `Set Enabled`)

(fn `Set Mask`
  (params (`Outline Mask` :type Integer))
  (bind _dynamic_outline_material (`self.Dynamic Outline Material`))
  (bind _output_get (set `self.Outline Mask` `Outline Mask`))
  (`/Engine/EditorBlueprintResources/StandardMacros.IsValid` _dynamic_outline_material
    (:`Is Valid`
      (message `AudioParameterControllerInterface.SetFloatParameter` _dynamic_outline_material (`self.Outline Mask Parameter Name`) (`KismetMathLibrary.Conv_IntToDouble` _output_get)))))

(fn `UserConstructionScript`)