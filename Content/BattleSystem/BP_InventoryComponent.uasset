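; Inventory component for the battle system that tracks owned items as a map from item class to quantity.
; AddItem stacks amounts with optional debug printing, while RemoveItem subtracts only when HasItem confirms enough are owned, returning success or failure.
; Save and Load hand the component to the save game object, with loading on BeginPlay when SaveGame is enabled.
; List prints each item's name and count.
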(event `self.ReceiveBeginPlay`
  (if (`self.bSaveGame`)
    (`self.Load`)))

(fn `AddItem`
  (params (Item :type "/Game/BattleSystem/Items/ItemBase Class Reference") (Amount :type Integer))
  (bind _item (`local.Item`))
  (bind (_value _returnvalue) (`BlueprintMapLibrary.Map_Find` (`self.Items`) Item))
  (bind _itemdetails_itemname (break `/Game/BattleSystem/Items/ItemDetailsStruct` (defaults `Object` _item)))
  (if _returnvalue
    (`BlueprintMapLibrary.Map_Add` (`self.Items`) (`local.Item`) (+ _value Amount))
    (else
      (`BlueprintMapLibrary.Map_Add` (`self.Items`) (`local.Item`) Amount)))
  (if (`self.Debug`)
    (`KismetSystemLibrary.PrintText` (`|FormatText` "adding {amount} of {item} ({total})" (`local.Amount`) _itemdetails_itemname (`BlueprintMapLibrary.Map_Find` (`self.Items`) _item)))))

(fn `HasItem`
  (params (Item :type "/Game/BattleSystem/Items/ItemBase Class Reference") (Amount :type Integer))
  (returns (Result :type Boolean) (`Owned Amount` :type Integer))
  (bind (_value _returnvalue) (`BlueprintMapLibrary.Map_Find` (`self.Items`) Item))
  (if _returnvalue
    (return (>= _value Amount) _value)
    (else
      (return false 0))))

(fn `List`
  (bind _keys (`BlueprintMapLibrary.Map_Keys` (`self.Items`)))
  (for _array_element _keys
    (bind _itemdetails_itemname (break `/Game/BattleSystem/Items/ItemDetailsStruct` (defaults `Object` _array_element)))
    (`KismetSystemLibrary.PrintText` (`|FormatText` "{amount} of {item}" (`BlueprintMapLibrary.Map_Find` (`self.Items`) _array_element) _itemdetails_itemname))))

(fn `Load`
  (bind (_success _savegameobject) (`/Game/BattleSystem/Data/JRPGLibrary.GetSaveFile`))
  (if _success
    (`/Game/BattleSystem/SaveGameData.LoadInventory` _savegameobject self)))

(fn `RemoveItem`
  (params (Item :type "/Game/BattleSystem/Items/ItemBase Class Reference") (Amount :type Integer))
  (returns (Result :type Boolean))
  (bind (_result _owned_amount) (`self.HasItem` Item Amount))
  (if _result
    (`BlueprintMapLibrary.Map_Add` (`self.Items`) (`local.Item`) (- _owned_amount Amount))
    (return true)
    (else
      (return false))))

(fn `Save`
  (bind (_success _savegameobject) (`/Game/BattleSystem/Data/JRPGLibrary.GetSaveFile`))
  (if _success
    (`/Game/BattleSystem/SaveGameData.SaveInventory` _savegameobject self)
    (`KismetSystemLibrary.PrintString` "inventory saved")))