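; Player controller for the battle system that owns the player's party of member actors.
; BeginPlay switches to game-only input and hides the mouse cursor.
; Party functions add, remove, list and look up members by their Info, with removal also destroying the actor.
; Adding or removing a member calls the PartyUpdated dispatcher to notify listeners.
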(event `self.ReceiveBeginPlay`
  (`WidgetBlueprintLibrary.SetInputMode_GameOnly` self)
  (set `self.bShowMouseCursor` false))

(fn `AddPartyMember`
  (params (Member :type "/Game/BattleSystem/Overworld/Party/PartyFollow Object Reference (by ref)"))
  (`KismetArrayLibrary.Array_Add` (`self.PartyMembers`) Member)
  (`self.PartyUpdated` self))

(fn `GetPartyMembers`
  (returns (Members :type "Array of /Game/BattleSystem/PartyMemberInfo Object Reference"))
  (locals (Info :type "Array of /Game/BattleSystem/PartyMemberInfo Object Reference"))
  (for _array_element (`self.PartyMembers`)
    (`KismetArrayLibrary.Array_Add` (`local.Info`) (`/Game/BattleSystem/Overworld/Party/PartyFollow.Info` _array_element)))
  (return (`local.Info`)))

(fn `HasPartyMember`
  (params (Info :type "/Game/BattleSystem/PartyMemberInfo Object Reference"))
  (returns (Result :type Boolean))
  (for _array_element (`self.PartyMembers`)
    (if (== (`/Game/BattleSystem/Overworld/Party/PartyFollow.Info` _array_element) (`local.Info`))
      (return true)))
  (return false))

(fn `RemovePartyMember`
  (params (Info :type "/Game/BattleSystem/PartyMemberInfo Object Reference (by ref)"))
  (for (_array_element _array_index) (`self.PartyMembers`)
    (if (== (`/Game/BattleSystem/Overworld/Party/PartyFollow.Info` _array_element) (`local.Info`))
      (`self.K2_DestroyActor` _array_element)
      (`KismetArrayLibrary.Array_Remove` (`self.PartyMembers`) _array_index)))
  (`self.PartyUpdated` self))

(fn `UserConstructionScript`)