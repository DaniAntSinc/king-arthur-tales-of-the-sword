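; Overworld Questing Beast NPC that removes itself based on the saved objective status.
; If SaveSlot1 exists, it loads the save as SaveGameData and switches on ObjectiveStatus, with every wired branch, including default, destroying the actor.
; BeginPlay, actor overlap and Tick all share this check, so the save is reloaded from the slot every frame.
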(event `self.ReceiveBeginPlay`
  (bind _returnvalue (`GameplayStatics.DoesSaveGameExist` "SaveSlot1" :!label _label))
  (if _returnvalue
    (bind _returnvalue_2 (`GameplayStatics.LoadGameFromSlot` "SaveSlot1"))
    (bind _assave_game_data (cast `/Game/BattleSystem/SaveGameData` _returnvalue_2))
    (switch `int` (`/Game/BattleSystem/SaveGameData.ObjectiveStatus` _assave_game_data)
      (:`Default`
        _)
      (:`0`
        _)
      (:`2`
        _))
    (`self.K2_DestroyActor`)))

(event `self.ReceiveActorBeginOverlap`
  (params (OtherActor :type "Actor Object Reference"))
  (`parent.ReceiveActorBeginOverlap` OtherActor)
  (goto _label))

(event `self.ReceiveTick`
  (params (DeltaSeconds :type "Float (single-precision)"))
  (`parent.ReceiveTick` DeltaSeconds)
  (goto _label))

(fn `UserConstructionScript`
  (`parent.UserConstructionScript`))