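; BP_NPC_Enemy_Interactable is an overworld enemy NPC that the player can interact with.
; Its sphere overlap registers it with the other actor's InteractorComponent and toggles a prompt widget, which is configured with an input action and description on BeginPlay.
; On interaction it calls an enemy-destroyed event, passes the interactor's owner to EnemyPlayerInformationComponent.PlayerOverlapped, then destroys itself.
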(event `self.ReceiveBeginPlay`
  (`parent.ReceiveBeginPlay`)
  (`self.SetupEnhancedInputAction`))

(event `self.Sphere.OnComponentBeginOverlap`
  (params (OverlappedComponent :type "PrimitiveComponent Object Reference") (OtherActor :type "Actor Object Reference") (OtherComp :type "PrimitiveComponent Object Reference") (OtherBodyIndex :type Integer) (bFromSweep :type Boolean) (SweepResult :type "HitResult Structure (by ref)"))
  (bind _returnvalue (`self.GetComponentByClass` OtherActor "/Game/BattleSystem/InteractorComponent.InteractorComponent_C"))
  (`/Engine/EditorBlueprintResources/StandardMacros.IsValid` _returnvalue
    (:`Is Valid`
      (`/Game/BattleSystem/InteractorComponent.AddInteractable` _returnvalue self)
      (`SceneComponent.SetVisibility` (`self.Widget`) true true))))

(event `self.Sphere.OnComponentEndOverlap`
  (params (OverlappedComponent :type "PrimitiveComponent Object Reference") (OtherActor :type "Actor Object Reference") (OtherComp :type "PrimitiveComponent Object Reference") (OtherBodyIndex :type Integer))
  (bind _returnvalue (`self.GetComponentByClass` OtherActor "/Game/BattleSystem/InteractorComponent.InteractorComponent_C"))
  (`/Engine/EditorBlueprintResources/StandardMacros.IsValid` _returnvalue
    (:`Is Valid`
      (`/Game/BattleSystem/InteractorComponent.RemoveInteractable` _returnvalue self)
      (`SceneComponent.SetVisibility` (`self.Widget`) false true))))

(event `/Game/BattleSystem/InteractableInterface.Interact`
  (params (Interactor :type "/Game/BattleSystem/InteractorComponent Object Reference"))
  (`self.EnemyDestroyedEvent` self)
  (`/Game/BattleSystem/Overworld/Enemies/AI/EnemyPlayerInformationComponent.PlayerOverlapped` (`self.EnemyPlayerInformationComponent`) (`ActorComponent.GetOwner` Interactor))
  (`self.K2_DestroyActor`))

(fn `GetActor`
  (returns (Actor :type "Actor Object Reference"))
  (return self))

(fn `SetupEnhancedInputAction`
  (bind _asinteraction_widget (cast `/Game/BattleSystem/UI/Widgets/Overworld/InteractionWidget` (`WidgetComponent.GetWidget` (`self.Widget`))))
  (`/Game/BattleSystem/UI/Widgets/Overworld/InteractionWidget.SetEnhancedInputAction` _asinteraction_widget (`self.InputAction`) (`self.Description`)))

(fn `UserConstructionScript`
  (`KismetSystemLibrary.PrintString` "I've Spawned" false true (struct :`R` 1.0 :`G` 0.01485 :`A` 1.0) 5.0))