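; BP_AIEnemyBase is the base overworld enemy in the battle system, reacting when the player touches it.
; When its sphere overlaps the player pawn, it calls the enemy-destroyed event, passes the pawn to its EnemyPlayerInformationComponent, then destroys itself.
; The construction script prints an on-screen spawn debug message.
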(event `self.Sphere.OnComponentBeginOverlap`
  (params (OverlappedComponent :type "PrimitiveComponent Object Reference") (OtherActor :type "Actor Object Reference") (OtherComp :type "PrimitiveComponent Object Reference") (OtherBodyIndex :type Integer) (bFromSweep :type Boolean) (SweepResult :type "HitResult Structure (by ref)"))
  (if (== OtherActor (`GameplayStatics.GetPlayerPawn` 0))
    (`self.EnemyDestroyedEvent` self)
    (`/Game/BattleSystem/Overworld/Enemies/EnemyPlayerInformationComponent.PlayerOverlapped` (`self.EnemyPlayerInformationComponent`) (`GameplayStatics.GetPlayerPawn` 0))
    (`self.K2_DestroyActor`)))

(fn `UserConstructionScript`
  (`KismetSystemLibrary.PrintString` "I've Spawned" true true (struct :`R` 1.0 :`G` 0.01485 :`A` 1.0) 5.0))